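; BP_CameraPawn is a pawn with mouse and gamepad look controls for a spring-arm camera rig.
; Horizontal input yaws the static mesh, while vertical input pitches the spring arm, then resets its rotation to a clamped target pitch with zero yaw and roll.
; Tick writes player pawn 0's transform into a camera pose from freshly made evaluation data, which is not applied further here.
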(event EventTick
  (params (DeltaSeconds :type Float%20%28single-precision%29))
  (Class|BlueprintCameraPoseFunctionLibrary|SetTransform (Class|BlueprintCameraEvaluationDataFunctionLibrary|GetCameraPose (Class|BlueprintCameraEvaluationDataFunctionLibrary|MakeCameraEvaluationData)) (Transformation|GetActorTransform (Game|Player|GetPlayerPawn 0))))

(event Input|MouseEvents|MouseY
  (params (AxisValue :type Float%20%28single-precision%29))
  (Transformation|AddLocalRotation (Variables|Default|GetSpringArm) (Math|Rotator|MakeRotator 0.0 AxisValue 0.0) false false)
  (Transformation|SetRelativeRotation (Variables|Default|GetSpringArm) (Math|Rotator|MakeRotator 0.0 (Math|Float|ClampAngle (.Pitch (Math|Rotator|BreakRotator (Class|SpringArmComponent|GetTargetRotation (Variables|Default|GetSpringArm)))) 45.0 2e+01) 0.0) false false))

(event Input|MouseEvents|MouseX
  (params (AxisValue :type Float%20%28single-precision%29))
  (Transformation|AddLocalRotation (Variables|Default|GetStaticMesh) (Math|Rotator|MakeRotator 0.0 0.0 AxisValue) false false))

(event Input|GamepadEvents|GamepadRightY
  (params (AxisValue :type Float%20%28single-precision%29))
  (Transformation|AddLocalRotation (Variables|Default|GetSpringArm) (Math|Rotator|MakeRotator 0.0 AxisValue 0.0) false false)
  (Transformation|SetRelativeRotation (Variables|Default|GetSpringArm) (Math|Rotator|MakeRotator 0.0 (Math|Float|ClampAngle (.Pitch (Math|Rotator|BreakRotator (Class|SpringArmComponent|GetTargetRotation (Variables|Default|GetSpringArm)))) 45.0 2e+01) 0.0) false false))

(event Input|GamepadEvents|GamepadRightX
  (params (AxisValue :type Float%20%28single-precision%29))
  (Transformation|AddLocalRotation (Variables|Default|GetStaticMesh) (Math|Rotator|MakeRotator 0.0 0.0 AxisValue) false false))

(fn ConstructionScript)